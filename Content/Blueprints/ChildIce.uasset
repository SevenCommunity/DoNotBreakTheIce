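; ChildIce is a child Blueprint for a damageable actor that awards score to the player when destroyed.
; On any damage it sets Health to Damage minus Health, and at zero or below it destroys itself and sends a score interface message to the player pawn.
; Its construction script runs the parent's, then randomizes the "rprm" scalar material parameter on the Cube for visual variation.
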(event EventBeginPlay)

(event Collision|EventActorBeginOverlap
  (params (OtherActor :type Actor%20Object%20Reference)))

(event EventTick
  (params (DeltaSeconds :type Float%20%28single-precision%29)))

(event Game|Damage|EventAnyDamage
  (params (Damage :type Float%20%28single-precision%29) (DamageType :type Damage%20Type%20Object%20Reference) (InstigatedBy :type Controller%20Object%20Reference) (DamageCauser :type Actor%20Object%20Reference))
  (bind _output_get (Variables|Default|SetHealth (- Damage (Variables|Default|GetHealth))))
  (if (<= _output_get 0.0)
    (Actor|DestroyActor)
    (Class|MyInterface|ScoreIT(Message) (Game|Player|GetPlayerPawn 0) 5.0)))

(fn ConstructionScript
  (|CallParentFunction)
  (Rendering|Material|SetScalarParameterValueonMaterials (Variables|Default|GetCube) "rprm" (Math|Random|RandomFloatinRange 0.2 0.7)))