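; Player pawn for a local turn-based hammer game where players take turns smashing MasterCubes for score.
; A cursor-following decal aims; one click starts a looping power bar, the next swings the hammer.
; Two overlap volumes highlight cubes in two tiers, which take power-scaled damage before the turn passes.
; It also handles right-mouse rotation, countdown and score widgets, and a Lose event that announces a winner other than the current player.
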(event OnComponentBeginOverlap(V0)
  (params (OverlappedComponent :type Primitive%20Component%20Object%20Reference) (OtherActor :type Actor%20Object%20Reference) (OtherComp :type Primitive%20Component%20Object%20Reference) (OtherBodyIndex :type Integer) (bFromSweep :type Boolean) (SweepResult :type Hit%20Result%20Structure%20%28by%20ref%29))
  (bind _targetcubesrange0 (Variables|Default|GetTargetCubesRange0))
  ;[0.09432 1 0] FIRST VOLUME COLLISION EVENTS
  (for _array_element (Collision|GetOverlappingActors (Variables|Default|GetV0) "/Game/Blueprints/MasterCube.MasterCube_C" :!class /Script/Engine.PrimitiveComponent)
    (bind _asmaster_cube (Utilities|Casting|CastToMasterCube _array_element))
    (if (not (Utilities|Array|ContainsItem _targetcubesrange0 _asmaster_cube))
      (Utilities|Array|Add _targetcubesrange0 _asmaster_cube)
      (Rendering|Material|SetVectorParameterValueonMaterials (Variables|/Game/Blueprints/MasterCube.MasterCube_C|GetCube _asmaster_cube) "Color" "5.000000,0.000000, 0")
      (Utilities|Array|RemoveItem (Variables|Default|GetTargetCubesRange1) _asmaster_cube))))

(event OnComponentBeginOverlap(V1)
  (params (OverlappedComponent :type Primitive%20Component%20Object%20Reference) (OtherActor :type Actor%20Object%20Reference) (OtherComp :type Primitive%20Component%20Object%20Reference) (OtherBodyIndex :type Integer) (bFromSweep :type Boolean) (SweepResult :type Hit%20Result%20Structure%20%28by%20ref%29))
  (bind _targetcubesrange1 (Variables|Default|GetTargetCubesRange1))
  ;[0.707 1 0] SECOND VOLUME COLLISION EVENTS
  (Utilities|FlowControl|Delay 0.1)
  (for _array_element (Collision|GetOverlappingActors (Variables|Default|GetV1) "/Game/Blueprints/MasterCube.MasterCube_C" :!class /Script/Engine.PrimitiveComponent)
    (bind _asmaster_cube (Utilities|Casting|CastToMasterCube _array_element))
    (if (not (or (Utilities|Array|ContainsItem (Variables|Default|GetTargetCubesRange0) _asmaster_cube) (Utilities|Array|ContainsItem _targetcubesrange1 _asmaster_cube)))
      (Utilities|Array|Add _targetcubesrange1 _asmaster_cube)
      (Rendering|Material|SetVectorParameterValueonMaterials (Variables|/Game/Blueprints/MasterCube.MasterCube_C|GetCube _asmaster_cube) "Color" "1.800000,0.900000,0.100000"))))

(event OnComponentEndOverlap(V1)
  (params (OverlappedComponent :type Primitive%20Component%20Object%20Reference) (OtherActor :type Actor%20Object%20Reference) (OtherComp :type Primitive%20Component%20Object%20Reference) (OtherBodyIndex :type Integer))
  (bind _targetcubesrange1 (Variables|Default|GetTargetCubesRange1))
  ;[0.707 1 0] SECOND VOLUME COLLISION EVENTS
  (for _array_element _targetcubesrange1
    (if (not (Utilities|Array|ContainsItem (Collision|GetOverlappingActors (Variables|Default|GetV1) "/Game/Blueprints/MasterCube.MasterCube_C" :!class /Script/Engine.PrimitiveComponent) _array_element))
      (Rendering|Material|SetVectorParameterValueonMaterials (Variables|/Game/Blueprints/MasterCube.MasterCube_C|GetCube _array_element) "Color" "0.086000,1.000000,1.000000")
      (Utilities|Array|RemoveItem _targetcubesrange1 _array_element))))

(event OnComponentEndOverlap(V0)
  (params (OverlappedComponent :type Primitive%20Component%20Object%20Reference) (OtherActor :type Actor%20Object%20Reference) (OtherComp :type Primitive%20Component%20Object%20Reference) (OtherBodyIndex :type Integer))
  (bind _targetcubesrange0 (Variables|Default|GetTargetCubesRange0))
  ;[0.09432 1 0] FIRST VOLUME COLLISION EVENTS
  (for _array_element _targetcubesrange0
    (if (not (Utilities|Array|ContainsItem (Collision|GetOverlappingActors (Variables|Default|GetV0) "/Game/Blueprints/MasterCube.MasterCube_C" :!class /Script/Engine.PrimitiveComponent) _array_element))
      (Rendering|Material|SetVectorParameterValueonMaterials (Variables|/Game/Blueprints/MasterCube.MasterCube_C|GetCube _array_element) "Color" "0.086000,1.000000,1.000000")
      (Utilities|Array|RemoveItem _targetcubesrange0 _array_element))))

(event Custom|hammerGO
  (bind _igref (Variables|Default|GetIGRef))
  (bind _igref_2 (Variables|Default|GetIGRef))
  (bind _hammer (Variables|Default|GetHammer))
  (bind _igref_3 (Variables|Default|GetIGRef))
  (bind _sctext (Variables|/Game/Blueprints/IGWidget.IGWidget_C|GetSCtext _igref))
  (bind _powerbar (Variables|/Game/Blueprints/IGWidget.IGWidget_C|Getpowerbar _igref_3))
  (bind _relativerotation (Variables|/Script/Engine.SceneComponent|GetRelativeRotation _hammer))
  (bind (_roll _pitch _yaw) (Math|Rotator|BreakRotator _relativerotation))
  (bind _percent (Variables|/Script/UMG.ProgressBar|GetPercent _powerbar))
  ;[1 0.04473 0.4899] HAMMER SMASH ( CUSTOM EVENT ) + APPLY DAMAGE TO CUBES :D
  (Rendering|SetVisibility (Variables|Default|GetHammer) true false)
  (bind _newtrack_0 (Timeline|HammerDriver PlayFromStart)
    (:Update
      (Transformation|SetRelativeRotation (Variables|Default|GetHammer) (Math|Interpolation|RInterpTo _relativerotation (Math|Rotator|MakeRotator (+ _roll 18.0) _pitch _yaw) _newtrack_0 0.1) false false))
    (:Finished
      (for _array_element (Variables|Default|GetTargetCubesRange0)
        (Game|Damage|ApplyDamage _array_element _percent 0 0))
      (for _array_element_2 (Variables|Default|GetTargetCubesRange1)
        (Game|Damage|ApplyDamage _array_element_2 (* _percent 5e+01) 0 0))
      (Utilities|FlowControl|Delay 1.0)
      (if (not (Variables|Default|Getend?))
        (bind _output_get (Variables|Default|SetCurrentPlayer (+ (Variables|Default|GetCurrentPlayer) 1)))
        (if (== (Math|Conversions|ToByte(Integer) (Utilities|Array|Length (Variables|Default|GetPlayers))) _output_get)
          (Variables|Default|SetCurrentPlayer 0))
        (Rendering|Components|TextRender|SetText _sctext (Utilities|Text|ToText(String) (Utilities|String|Append "Player : " (Utilities|String|ToString(Byte) (.id (Utilities|Struct|BreakPlayerStruct (Utilities|Array|Get(acopy) (Variables|Default|GetPlayers) (Math|Conversions|ToInteger(Byte) (Variables|Default|GetCurrentPlayer)))))) " Turn !")))
        (Appearance|SetColorandOpacity _sctext (Utilities|Struct|MakeSlateColor (.assoc_color (Utilities|Struct|BreakPlayerStruct (Utilities|Array|Get(acopy) (Variables|Default|GetPlayers) (Math|Conversions|ToInteger(Byte) (Variables|Default|GetCurrentPlayer))))) "UseColor_Specified") :!class /Script/UMG.TextBlock)
        (UserInterface|Animation|PlayAnimation _igref_2 (Variables|/Game/Blueprints/IGWidget.IGWidget_C|Gettextanim _igref_2) 0.0 1 "Forward" 1.0)))))

(event EventTick
  (params (DeltaSeconds :type Float%20%28single-precision%29))
  (bind _returnvalue (Game|GetPlayerController 0))
  (bind _igref (Variables|Default|GetIGRef))
  (bind _hitresult (Game|Player|GetHitResultUnderCursorbyChannel _returnvalue "TraceTypeQuery1" true))
  (bind _powerbar (Variables|/Game/Blueprints/IGWidget.IGWidget_C|Getpowerbar _igref))
  (bind (_bblockinghit _binitialoverlap _time _location _impactpoint _normal _impactnormal) (Collision|BreakHitResult _hitresult))
  (bind _percent (Variables|/Script/UMG.ProgressBar|GetPercent _powerbar))
  ;[0 0.3171 1] EVENT TICK : (1) Decale Followiing mouse , (2) PowerBar Hammer Charge
  (if (not (Variables|Default|Getend?))
    (Transformation|SetWorldLocationAndRotation (Variables|Default|GetMouseDec) _location (Math|Rotator|MakeRotationfromAxes _impactnormal "0, 0, 0" "0, 0, 0") false false)
    (Utilities|FlowControl|Gate true
      (:Exit
        (Progress|SetPercent _powerbar (+ _percent 0.02))
        (if (>= _percent 1.0)
          (Progress|SetPercent _powerbar 0.0))))))

(event EventScoreIT
  (params (score :type Float%20%28single-precision%29))
  (bind _players (Variables|Default|GetPlayers))
  (bind _currentplayer (Variables|Default|GetCurrentPlayer))
  (bind _returnvalue (Math|Conversions|ToInteger(Byte) _currentplayer))
  (bind _output (Utilities|Array|Get(acopy) _players _returnvalue))
  (bind (_id _assoc_color _score _assoc_subwid) (Utilities|Struct|BreakPlayerStruct _output))
  ;[1 0 0] score increase
  (bind _structout (Utilities|Struct|SetmembersinPlayerStruct (Utilities|Struct|MakePlayerStruct _id _assoc_color (+ (Math|Float|Truncate score) _score) _assoc_subwid)))
  (Utilities|Array|SetArrayElem _players _returnvalue _structout)
  (Rendering|Components|TextRender|SetText (Variables|/Game/Blueprints/PlayerStateWID.PlayerStateWID_C|Getscoretext (.assoc_subwid (Utilities|Struct|BreakPlayerStruct _structout))) (Utilities|Text|ToText(Integer) (.Score (Utilities|Struct|BreakPlayerStruct _structout)))))

(event EventLose
  (bind _igref (Variables|Default|GetIGRef))
  (bind _igref_2 (Variables|Default|GetIGRef))
  (bind _sctext (Variables|/Game/Blueprints/IGWidget.IGWidget_C|GetSCtext _igref))
  ;[1 0 0] Player lose
  (bind _output_get (CallFunction|GetWinner))
  (Rendering|Components|TextRender|SetText _sctext (Utilities|Text|ToText(String) (Utilities|String|Append "Player :" (Utilities|String|ToString(Byte) (.id (Utilities|Struct|BreakPlayerStruct _output_get))) "won !" "(SCORE : " (Utilities|String|ToString(Integer) (.Score (Utilities|Struct|BreakPlayerStruct _output_get))) ")")))
  (Appearance|SetColorandOpacity _sctext (Utilities|Struct|MakeSlateColor (.assoc_color (Utilities|Struct|BreakPlayerStruct _output_get)) "UseColor_Specified") :!class /Script/UMG.TextBlock)
  (UserInterface|Animation|PlayAnimation _igref_2 (Variables|/Game/Blueprints/IGWidget.IGWidget_C|Gettextanim _igref_2) 0.0 1 "Forward" 1.0)
  (Variables|Default|Setend? true)
  (Utilities|FlowControl|Delay 3.0)
  (Widget|RemovefromParent (Variables|Default|GetIGRef))
  (bind _returnvalue (UserInterface|CreateWidget "/Game/Blueprints/NavigateUI.NavigateUI_C"))
  (UserInterface|Viewport|AddtoViewport _returnvalue 0))

(event EventBeginPlay
  (bind _players (Variables|Default|GetPlayers))
  (bind _players_2 (Variables|Default|GetPlayers))
  (bind _currentplayer (Variables|Default|GetCurrentPlayer))
  (bind _returnvalue (Math|Conversions|ToInteger(Byte) _currentplayer))
  (bind _output (Utilities|Array|Get(acopy) _players_2 _returnvalue))
  (bind (_id _assoc_color) (Utilities|Struct|BreakPlayerStruct _output))
  ;[1 0.319 0.3888] Init : (1) Mouse - (2) Create Widget
  (bind _asice_pcontrol (Utilities|Casting|CastToIcePControl (Game|GetPlayerController 0)))
  (bind _output_get (Variables|Default|SetPlayerCNRef _asice_pcontrol))
  (Input|DisableInput _output_get)
  (Variables|/Script/Engine.PlayerController|SetbShowMouseCursor _output_get true)
  (bind _returnvalue_2 (UserInterface|CreateWidget "/Game/Blueprints/IGWidget.IGWidget_C"))
  (bind _output_get_2 (Variables|Default|SetIGRef _returnvalue_2))
  (UserInterface|Viewport|AddtoViewport _output_get_2 0)
  (for (_array_element _array_index) _players
    (bind _returnvalue_3 (UserInterface|CreateWidget "/Game/Blueprints/PlayerStateWID.PlayerStateWID_C"))
    (Class|VerticalBox|AddChildtoVerticalBox (Variables|/Game/Blueprints/IGWidget.IGWidget_C|GetVerticalBox_72 (Variables|Default|GetIGRef)) _returnvalue_3)
    (bind _structout (Utilities|Struct|SetmembersinPlayerStruct (Utilities|Struct|MakePlayerStruct (.id (Utilities|Struct|BreakPlayerStruct _array_element)) (.assoc_color (Utilities|Struct|BreakPlayerStruct _array_element)) (.Score (Utilities|Struct|BreakPlayerStruct _array_element)) _returnvalue_3)))
    (Utilities|Array|SetArrayElem _players _array_index _structout)
    (Rendering|Components|TextRender|SetText (Variables|/Game/Blueprints/PlayerStateWID.PlayerStateWID_C|Getplayeridtext _returnvalue_3) (Utilities|Text|ToText(String) (Utilities|String|Append "Player : " (Utilities|String|ToString(Byte) (.id (Utilities|Struct|BreakPlayerStruct _array_element))) " Score ")))
    (Rendering|Components|TextRender|SetText (Variables|/Game/Blueprints/PlayerStateWID.PlayerStateWID_C|Getscoretext _returnvalue_3) "0")
    (Appearance|SetColorandOpacity (Variables|/Game/Blueprints/PlayerStateWID.PlayerStateWID_C|Getplayeridtext _returnvalue_3) (Utilities|Struct|MakeSlateColor (.assoc_color (Utilities|Struct|BreakPlayerStruct _structout)) "UseColor_Specified") :!class /Script/UMG.TextBlock))
  (Rendering|Components|TextRender|SetText (Variables|/Game/Blueprints/IGWidget.IGWidget_C|GetSCtext (Variables|Default|GetIGRef)) (Utilities|Text|ToText(String) "Game starting in 3 seconds"))
  (Appearance|SetColorandOpacity (Variables|/Game/Blueprints/IGWidget.IGWidget_C|GetSCtext (Variables|Default|GetIGRef)) (Utilities|Struct|MakeSlateColor "(R=0.000000,G=1.000000,B=0.959561,A=1.000000)") :!class /Script/UMG.TextBlock)
  (UserInterface|Animation|PlayAnimation (Variables|Default|GetIGRef) (Variables|/Game/Blueprints/IGWidget.IGWidget_C|Gettextanim (Variables|Default|GetIGRef)) 0.0 1 "Forward" 1.0)
  (Utilities|FlowControl|Delay 2.0)
  ;;[0.1366 0 1] Countdown animatoin
  (Utilities|DirectText (Variables|Default|GetIGRef) (Variables|/Game/Blueprints/IGWidget.IGWidget_C|GetCount (Variables|Default|GetIGRef)) (Variables|/Game/Blueprints/IGWidget.IGWidget_C|GetSCtext (Variables|Default|GetIGRef)) "0" "(R=0.000000,G=0.000000,B=0.000000,A=1.000000)")
  (Utilities|DirectText (Variables|Default|GetIGRef) (Variables|/Game/Blueprints/IGWidget.IGWidget_C|GetCount (Variables|Default|GetIGRef)) (Variables|/Game/Blueprints/IGWidget.IGWidget_C|GetSCtext (Variables|Default|GetIGRef)) "1")
  (Utilities|DirectText (Variables|Default|GetIGRef) (Variables|/Game/Blueprints/IGWidget.IGWidget_C|GetCount (Variables|Default|GetIGRef)) (Variables|/Game/Blueprints/IGWidget.IGWidget_C|GetSCtext (Variables|Default|GetIGRef)) "2")
  (Utilities|DirectText (Variables|Default|GetIGRef) (Variables|/Game/Blueprints/IGWidget.IGWidget_C|GetCount (Variables|Default|GetIGRef)) (Variables|/Game/Blueprints/IGWidget.IGWidget_C|GetSCtext (Variables|Default|GetIGRef)) "3")
  (Utilities|DirectText (Variables|Default|GetIGRef) (Variables|/Game/Blueprints/IGWidget.IGWidget_C|GetCount (Variables|Default|GetIGRef)) (Variables|/Game/Blueprints/IGWidget.IGWidget_C|GetSCtext (Variables|Default|GetIGRef)) (Utilities|Text|ToText(String) (Utilities|String|Append "Player : " (Utilities|String|ToString(Byte) _id) " Turn !")) _assoc_color)
  (Input|EnableInput (Variables|Default|GetPlayerCNRef))
  (Utilities|FlowControl|Delay 2.0)
  (UserInterface|Animation|PlayAnimation (Variables|Default|GetIGRef) (Variables|/Game/Blueprints/IGWidget.IGWidget_C|Gettextanim (Variables|Default|GetIGRef)) 0.0 1 "Reverse" 1.0))

(event Input|AxisEvents|InputAxisTurn
  (params (AxisValue :type Float%20%28single-precision%29))
  ;[0.1274 1 0.6626] Mouse input + rotation handle
  (Utilities|FlowControl|Gate true
    (:Exit
      (|SetMouse50%
        (:then2
          (Pawn|Input|AddControllerYawInput AxisValue))))))

(event Input|MouseEvents|LeftMouseButton
  (params (Key :type Key%20Structure))
  (bind _mousedec (Variables|Default|GetMouseDec))
  (bind _igref (Variables|Default|GetIGRef))
  (bind _camera (Variables|Default|GetCamera))
  (bind _returnvalue (Transformation|GetWorldLocation _camera))
  (bind _returnvalue_2 (Transformation|GetWorldLocation _mousedec))
  (bind _powerbar (Variables|/Game/Blueprints/IGWidget.IGWidget_C|Getpowerbar _igref))
  (bind _returnvalue_3 (Math|Rotator|FindLookatRotation _returnvalue _returnvalue_2))
  (bind (_x _y _z) (Math|Vector|BreakVector _returnvalue_2))
  (bind _percent (Variables|/Script/UMG.ProgressBar|GetPercent _powerbar))
  ;[0 0.3171 1] EVENT TICK : (1) Decale Followiing mouse , (2) PowerBar Hammer Charge
  (:Pressed
    (if (> (Utilities|Array|Length (Variables|Default|GetTargetCubesRange0)) 0)
      (Transformation|SetWorldLocationAndRotation (Variables|Default|GetHammer) (Math|Vector|MakeVector _x _y (+ _z 5e+01)) (Math|Rotator|MakeRotator (.roll _returnvalue_3) (.pitch (Variables|Default|GetinitROT)) (.yaw _returnvalue_3)) false false)
      (if (Variables|Default|GetCH)
        (Variables|Default|SetCH false)
        (CallFunction|HammerGO)
        (Utilities|FlowControl|Gate true) ; enters at Close
        (else
          (Variables|Default|SetCH true)
          (Utilities|FlowControl|Gate true) ; enters at Open
        )))))

(event Input|MouseEvents|RightMouseButton
  (params (Key :type Key%20Structure))
  (bind _playercnref (Variables|Default|GetPlayerCNRef))
  (bind _v1 (Variables|Default|GetV1))
  ;[0.1274 1 0.6626] Mouse input + rotation handle
  (:Pressed
    (Variables|/Script/Engine.PlayerController|SetbShowMouseCursor _playercnref false)
    (Rendering|SetVisibility (Variables|Default|GetHammer) false false)
    (Collision|SetCollisionEnabled _v1 "NoCollision")
    (Utilities|FlowControl|Gate true) ; enters at Open
  )
  (:Released
    (Variables|/Script/Engine.PlayerController|SetbShowMouseCursor _playercnref true)
    (Collision|SetCollisionEnabled _v1 "QueryOnly")
    (Utilities|FlowControl|Gate true) ; enters at Close
  ))

(fn ConstructionScript
  (Variables|Default|SetinitROT (Variables|/Script/Engine.SceneComponent|GetRelativeRotation (Variables|Default|GetHammer))))

(fn GetWinner
  (for (_array_element _array_index) (Variables|Default|GetPlayers)
    (if (and (!= (Math|Conversions|ToByte(Integer) _array_index) (Variables|Default|GetCurrentPlayer)) (> (.Score (Utilities|Struct|BreakPlayerStruct _array_element)) (.Score (Utilities|Struct|BreakPlayerStruct (LocalVariables|GetwinnerID)))))
      (bind _output_get (LocalVariables|SetwinnerID _array_element))
      (return _output_get))))